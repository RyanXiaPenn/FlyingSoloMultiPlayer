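; LevelTrigger is a one-shot overlap trigger that extends the player's timer and removes level actors.
; When a StudentVRTest actor first overlaps it, it adds TimeAdded to that actor's TimeLeft.
; It then destroys the first actor found for each of two tags, SpawnToBeDestroyed and SpawnToBeDestroyed2, and plays a 2D explosion sound.
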(event `self.ReceiveActorBeginOverlap`
  (params (OtherActor :type "Actor Object Reference"))
  (if (`KismetMathLibrary.ClassIsChildOf` (`GameplayStatics.GetObjectClass` OtherActor) "/Game/Blueprints/StudentVRTest.StudentVRTest_C")
    (bind _asstudent_vrtest (cast `/Game/Blueprints/StudentVRTest` OtherActor))
    (`/Engine/EditorBlueprintResources/StandardMacros.DoOnce` false
      (:`Completed`
        (set `/Game/Blueprints/StudentVRTest.TimeLeft` (+ (`/Game/Blueprints/StudentVRTest.TimeLeft` _asstudent_vrtest) (`self.TimeAdded`)) _asstudent_vrtest)
        (bind _outactors (`GameplayStatics.GetAllActorsWithTag` (`self.SpawnToBeDestroyed`)))
        (`self.K2_DestroyActor` (`|GetArrayItem` _outactors))
        (bind _outactors_2 (`GameplayStatics.GetAllActorsWithTag` (`self.SpawnToBeDestroyed2`)))
        (`self.K2_DestroyActor` (`|GetArrayItem` _outactors_2))
        (`GameplayStatics.PlaySound2D` "/Game/StarterContent/Audio/Explosion01.Explosion01" 1.0 1.0 0.0 null null)))))

(fn `UserConstructionScript`)