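; Pencil2 is a VR pickup pencil that pops what it hits on StudentVRTest actors.
; Pickup, called by BP_MotionController, disables mesh physics and attaches the root to the given component, while Drop re-enables physics and detaches it.
; On a hit with a StudentVRTest-derived actor, it destroys the struck component and plays BalloonPop at the pencil's location.
; Leftover nodes for destroying the actor and spawning SteamBP are unconnected.
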(event `/Game/VirtualRealityBP/Blueprints/PickupActorInterface.Pickup`
  (params (AttachTo :type "SceneComponent Object Reference"))
  (`PrimitiveComponent.SetSimulatePhysics` (`self.StaticMeshComponent`) false)
  (`SceneComponent.K2_AttachToComponent` (`self.K2_GetRootComponent`) AttachTo "None" "KeepWorld" "KeepWorld" "KeepWorld" false))

(event `/Game/VirtualRealityBP/Blueprints/PickupActorInterface.Drop`
  (`PrimitiveComponent.SetSimulatePhysics` (`self.StaticMeshComponent`) true)
  (`self.K2_DetachFromActor` "KeepWorld" "KeepWorld" "KeepWorld"))

(event `self.ReceiveHit`
  (params (MyComp :type "PrimitiveComponent Object Reference") (Other :type "Actor Object Reference") (OtherComp :type "PrimitiveComponent Object Reference") (bSelfMoved :type Boolean) (HitLocation :type "Vector Structure") (HitNormal :type "Vector Structure") (NormalImpulse :type "Vector Structure") (Hit :type "HitResult Structure (by ref)"))
  (if (`KismetMathLibrary.ClassIsChildOf` (`GameplayStatics.GetObjectClass` Other) "/Game/Blueprints/StudentVRTest.StudentVRTest_C")
    (`ActorComponent.K2_DestroyComponent` OtherComp)
    (`GameplayStatics.PlaySoundAtLocation` "/Game/Audio/BalloonPop.BalloonPop" (`self.K2_GetActorLocation`) (struct) 1.0 1.0 0.0 null null null)))

(fn `UserConstructionScript`)