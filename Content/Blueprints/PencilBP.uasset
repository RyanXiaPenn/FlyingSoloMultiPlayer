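; PencilBP is a VR pencil that the player picks up and uses to pop YellowEnemy actors for bonus time.
; Pickup, called by BP_MotionController, disables physics and attaches it to the given component, while Drop re-enables physics and detaches it.
; Hitting a YellowEnemy destroys both actors, plays a balloon pop, spawns SteamBP and adds to TimeLeft on the first StudentVRTest found in the level.
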(event `/Game/VirtualRealityBP/Blueprints/PickupActorInterface.Pickup`
  (params (AttachTo :type "SceneComponent Object Reference"))
  (`PrimitiveComponent.SetSimulatePhysics` (`self.StaticMeshComponent`) false)
  (`SceneComponent.K2_AttachToComponent` (`self.K2_GetRootComponent`) AttachTo "None" "KeepWorld" "KeepWorld" "KeepWorld" false))

(event `/Game/VirtualRealityBP/Blueprints/PickupActorInterface.Drop`
  (`PrimitiveComponent.SetSimulatePhysics` (`self.StaticMeshComponent`) true)
  (`self.K2_DetachFromActor` "KeepWorld" "KeepWorld" "KeepWorld"))

(event `self.ReceiveHit`
  (params (MyComp :type "PrimitiveComponent Object Reference") (Other :type "Actor Object Reference") (OtherComp :type "PrimitiveComponent Object Reference") (bSelfMoved :type Boolean) (HitLocation :type "Vector Structure") (HitNormal :type "Vector Structure") (NormalImpulse :type "Vector Structure") (Hit :type "HitResult Structure (by ref)"))
  (bind _returnvalue (`self.K2_GetActorLocation`))
  (if (`KismetMathLibrary.ClassIsChildOf` (`GameplayStatics.GetObjectClass` Other) "/Game/Blueprints/yellowEnemy.yellowEnemy_C")
    (`self.K2_DestroyActor` Other)
    (`GameplayStatics.PlaySoundAtLocation` "/Game/Audio/BalloonPop.BalloonPop" _returnvalue (struct) 1.0 1.0 0.0 null null null)
    (`self.K2_DestroyActor`)
    (`|SpawnActorFromClass` "/Game/Blueprints/SteamBP.SteamBP_C" (`KismetMathLibrary.Conv_VectorToTransform` _returnvalue) "Undefined" "OverrideRootScale" null null)
    (bind _outactors (`GameplayStatics.GetAllActorsOfClass` "/Game/Blueprints/StudentVRTest.StudentVRTest_C"))
    (bind _output (`|GetArrayItem` _outactors))
    (set `/Game/Blueprints/StudentVRTest.TimeLeft` (+ (`/Game/Blueprints/StudentVRTest.TimeLeft` _output) 5.0) _output)))

(fn `UserConstructionScript`)