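; RedEnemy is an enemy actor that BP_MotionController can pick up and drop.
; Pickup turns off mesh physics, attaches the root to the supplied component keeping world transform and plays a grab sound.
; Drop restores physics and detaches the actor.
; Tick resets the PhysicsThruster to a fixed world rotation, so its thrust direction stays constant however the actor turns.
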(event `self.ReceiveTick`
  (params (DeltaSeconds :type "Float (single-precision)"))
  (`SceneComponent.K2_SetWorldRotation` (`self.PhysicsThruster`) (struct :`Pitch` -90.0) false false))

(event `/Game/VirtualRealityBP/Blueprints/PickupActorInterface.Pickup`
  (params (AttachTo :type "SceneComponent Object Reference"))
  (`PrimitiveComponent.SetSimulatePhysics` (`self.StaticMeshComponent`) false)
  (`SceneComponent.K2_AttachToComponent` (`self.K2_GetRootComponent`) AttachTo "None" "KeepWorld" "KeepWorld" "KeepWorld" false)
  (`GameplayStatics.PlaySound2D` "/Game/Audio/grabSound.grabSound" 1.0 1.0 0.0 null null))

(event `/Game/VirtualRealityBP/Blueprints/PickupActorInterface.Drop`
  (`PrimitiveComponent.SetSimulatePhysics` (`self.StaticMeshComponent`) true)
  (`self.K2_DetachFromActor` "KeepWorld" "KeepWorld" "KeepWorld"))

(fn `UserConstructionScript`)