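; YellowBalloonSpawn is a spawner actor that continuously produces YellowEnemy actors around its own location for as long as it runs.
; BeginPlay starts an endless loop that spawns one enemy, waits a random delay of up to a few seconds, then repeats.
; Each spawn gets a small random horizontal offset at the spawner's height, a fully random rotation and a random per-axis scale, so enemies vary in shape and size.
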(event `self.ReceiveBeginPlay`
  (bind _returnvalue (`KismetMathLibrary.RandomFloatInRange` 0.8 1.5))
  (`|SpawnActorFromClass` "/Game/Blueprints/yellowEnemy.yellowEnemy_C" (`KismetMathLibrary.MakeTransform` (`KismetMathLibrary.MakeVector` (+ (.x (.location (`self.GetTransform`))) (`KismetMathLibrary.RandomFloatInRange` -80.0 80.0)) (+ (.y (.location (`self.GetTransform`))) (`KismetMathLibrary.RandomFloatInRange` -80.0 80.0)) (.z (.location (`self.GetTransform`)))) (`KismetMathLibrary.MakeRotator` (`KismetMathLibrary.RandomFloatInRange` -180.0 180.0) (`KismetMathLibrary.RandomFloatInRange` -180.0 180.0) (`KismetMathLibrary.RandomFloatInRange` -180.0 180.0)) (`KismetMathLibrary.MakeVector` _returnvalue _returnvalue (`KismetMathLibrary.RandomFloatInRange` 0.8 1.5))) "Undefined" "OverrideRootScale" null null :!label _label)
  (`KismetSystemLibrary.Delay` (`KismetMathLibrary.RandomFloatInRange` 0.4 5.0))
  (goto _label))

(fn `UserConstructionScript`)